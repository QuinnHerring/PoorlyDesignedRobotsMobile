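; Blue end zone actor that glows while the player pawn stands on it and always allows the player to enter.
; Each tick, after the parent logic, it compares its X and Y location to player pawn 0 using exact equality.
; A match switches both static meshes to the blue glow material; otherwise they use the base blue material.
; CanPlayerEnter returns true regardless of pawn or origin.
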(event EventBeginPlay
  (|CallParentFunction) ; This node is disabled and will not be called.\nDrag off pins to build functionality.
)

(event Collision|EventActorBeginOverlap
  (params (OtherActor :type Actor%20Object%20Reference))
  (|CallParentFunction OtherActor))

(event EventTick
  (params (DeltaSeconds :type Float%20%28single-precision%29))
  (bind _returnvalue (Game|Player|GetPlayerPawn 0))
  (bind _self self)
  (bind _returnvalue_2 (Transformation|GetActorLocation _returnvalue))
  (bind _returnvalue_3 (Transformation|GetActorLocation _self))
  (bind (_x _y) (Math|Vector|BreakVector _returnvalue_2))
  (bind (_x_2 _y_2) (Math|Vector|BreakVector _returnvalue_3))
  (|CallParentFunction DeltaSeconds)
  (if (and (== _x_2 _x) (== _y_2 _y))
    (Rendering|Material|SetMaterial (Variables|Default|GetStaticMesh) 0 "/Game/Meshes/Materials/EndZoneGlowBlue.EndZoneGlowBlue")
    (Rendering|Material|SetMaterial (Variables|Default|GetStaticMesh2) 0 "/Game/Meshes/Materials/EndZoneGlowBlue.EndZoneGlowBlue")
    (else
      (Rendering|Material|SetMaterial (Variables|Default|GetStaticMesh) 0 "/Game/Meshes/Materials/EndZoneBaseBlue.EndZoneBaseBlue")
      (Rendering|Material|SetMaterial (Variables|Default|GetStaticMesh2) 0 "/Game/Meshes/Materials/EndZoneBaseBlue.EndZoneBaseBlue"))))

(fn ConstructionScript
  (|CallParentFunction))

(fn CanPlayerEnter
  (params (Player%20Pawn :type Player%20Pawn%20Object%20Reference) (From :type Tile%20Object%20Reference))
  (return true))