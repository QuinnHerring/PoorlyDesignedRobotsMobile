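; Pressure plate that moves a linked bridge tile while pressed and moves it back when released.
; Press and release events swap the button's glow materials, restoring the off look from spare material slots.
; The tile's IsRaised flag gates each move, and its DirectionOfMovement selects the movement call or its opposite.
; Release waits a brief delay and rechecks IsPressed, so an immediate re-press cancels the reversal.
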(event Custom|Off%20Pressure%20Plate
  (bind _affectedbridgetile (Variables|Components|GetAffectedBridgeTile))
  (Variables|Default|SetisPressed false)
  ;[1 1 1] DO NOT REMOVE
  (Utilities|FlowControl|Delay 0.01)
  (if (not (Variables|Default|GetisPressed))
    ;[1 1 1] Sets "PressurePlate Off" Materials
    (Rendering|Material|SetMaterial (Variables|Default|GetButton) 1 (Rendering|Material|GetMaterial (Variables|Default|GetButton) 7))
    (Rendering|Material|SetMaterial (Variables|Default|GetButton) 2 (Rendering|Material|GetMaterial (Variables|Default|GetButton) 6))
    (Rendering|Material|SetMaterial (Variables|Default|GetButton) 3 (Rendering|Material|GetMaterial (Variables|Default|GetButton) 5))
    ;[1 1 1] Checks if bridge is in inverse position to its new position
    (if (Variables|/Game/Blueprints/Bridge.Bridge_C|GetisRaised (Variables|Components|GetAffectedBridgeTile))
      ;[1 1 1] Based on "Direction of Movement" do OPPOSITE bridge movement
      (switch string (Variables|/Game/Blueprints/Bridge.Bridge_C|GetDirection%20of%20Movement (Variables|Components|GetAffectedBridgeTile))
        (:Up
          (Default|DropBridge _affectedbridgetile))
        (:Down
          (Default|RaiseBridge _affectedbridgetile))
        (:Forwards
          (Default|MoveBridgeBackwards _affectedbridgetile))
        (:Back
          (Default|MoveBridgeForwards _affectedbridgetile))
        (:Left
          (Default|MoveBridgeRight _affectedbridgetile))
        (:Right
          (Default|MoveBridgeLeft _affectedbridgetile)))
      ;[1 1 1] Set if the bridge is raised/fallen
      (Variables|/Game/Blueprints/Bridge.Bridge_C|SetisRaised (Variables|Components|GetAffectedBridgeTile) false))))

(event Custom|On%20Pressure%20Plate
  (bind _affectedbridgetile (Variables|Components|GetAffectedBridgeTile))
  (Variables|Default|SetisPressed true)
  ;[1 1 1] Sets "Pressure Plate On" Materials
  (Rendering|Material|SetMaterial (Variables|Default|GetButton) 1 "/Game/Textures/Robots/EndZoneBlueGlow.EndZoneBlueGlow")
  (Rendering|Material|SetMaterial (Variables|Default|GetButton) 2 "/Game/Textures/Robots/EndZoneBlueGlow.EndZoneBlueGlow")
  (Rendering|Material|SetMaterial (Variables|Default|GetButton) 3 "/Game/Textures/Robots/EndZoneBlueGlow.EndZoneBlueGlow")
  ;[1 1 1] Checks if bridge is in inverse position to its new position
  (if (not (Variables|/Game/Blueprints/Bridge.Bridge_C|GetisRaised (Variables|Components|GetAffectedBridgeTile)))
    ;[1 1 1] Based on "Direction of Movement" do bridge movement
    (switch string (Variables|/Game/Blueprints/Bridge.Bridge_C|GetDirection%20of%20Movement (Variables|Components|GetAffectedBridgeTile))
      (:Up
        (Default|RaiseBridge _affectedbridgetile))
      (:Down
        (Default|DropBridge _affectedbridgetile))
      (:Forwards
        (Default|MoveBridgeForwards _affectedbridgetile))
      (:Back
        (Default|MoveBridgeBackwards _affectedbridgetile))
      (:Left
        (Default|MoveBridgeLeft _affectedbridgetile))
      (:Right
        (Default|MoveBridgeRight _affectedbridgetile)))
    ;[1 1 1] Set if the bridge is raised/fallen
    (Variables|/Game/Blueprints/Bridge.Bridge_C|SetisRaised (Variables|Components|GetAffectedBridgeTile) true)))

(fn ConstructionScript
  (|CallParentFunction))