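; Base tile actor for a 3D tile map, holding a grid coordinate, a map of neighbours by direction and player entry and occupancy checks.
; FindNeighbours looks up fourteen directions in the TileMap, including vertical and diagonal up/down ones.
; ChangeTileType replaces the tile with a spawned actor of the new class and relinks its neighbours.
; SwapTiles exchanges index and coordinates with an adjacent tile, then rebuilds surrounding neighbour links.
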(event EventBeginPlay)

(event Collision|EventActorBeginOverlap
  (params (OtherActor :type Actor%20Object%20Reference)))

(event EventTick
  (params (DeltaSeconds :type Float%20%28single-precision%29)))

(fn ConstructionScript)

(fn FindNeighbours
  (bind _coord (Variables|Default|GetCoord))
  (for _array_element (Utilities|Array|MakeArray "/Game/Blueprints/Forwards.Forwards" "/Game/Blueprints/Back.Back" "/Game/Blueprints/Left.Left" "/Game/Blueprints/Right.Right" "/Game/Blueprints/upForwards.UpForwards" "/Game/Blueprints/UpBack.UpBack" "/Game/Blueprints/UpLeft.UpLeft" "/Game/Blueprints/UpRight.UpRight" "/Game/Blueprints/DownForwards.DownForwards" "/Game/Blueprints/DownBack.DownBack" "/Game/Blueprints/DownLeft.DownLeft" "/Game/Blueprints/DownRight.DownRight" "/Game/Blueprints/Up.Up" "/Game/Blueprints/Down.Down")
    (if (Default|IsCoordinRange (Variables|Default|GetTile%20Map) (Utilities|Struct|MakeIntVector (+ (.x (Variables|/Game/Blueprints/Direction.Direction_C|GetDelta _array_element)) (.x _coord)) (+ (.y (Variables|/Game/Blueprints/Direction.Direction_C|GetDelta _array_element)) (.y _coord)) (+ (.z (Variables|/Game/Blueprints/Direction.Direction_C|GetDelta _array_element)) (.z _coord))))
      (Utilities|IsValid (Default|GetTileatCoord (Variables|Default|GetTile%20Map) (Utilities|Struct|MakeIntVector (+ (.x (Variables|/Game/Blueprints/Direction.Direction_C|GetDelta _array_element)) (.x _coord)) (+ (.y (Variables|/Game/Blueprints/Direction.Direction_C|GetDelta _array_element)) (.y _coord)) (+ (.z (Variables|/Game/Blueprints/Direction.Direction_C|GetDelta _array_element)) (.z _coord))))
        (:Is%20Valid
          (Utilities|Map|Add (Variables|Default|GetNeighbours) _array_element (Default|GetTileatCoord (Variables|Default|GetTile%20Map) (Utilities|Struct|MakeIntVector (+ (.x (Variables|/Game/Blueprints/Direction.Direction_C|GetDelta _array_element)) (.x _coord)) (+ (.y (Variables|/Game/Blueprints/Direction.Direction_C|GetDelta _array_element)) (.y _coord)) (+ (.z (Variables|/Game/Blueprints/Direction.Direction_C|GetDelta _array_element)) (.z _coord))))))))))

(fn SetNeighbour
  (params (Direction :type Direction%20Object%20Reference) (New%20Neighbour :type Tile%20Object%20Reference))
  (Utilities|Map|Add (Variables|Default|GetNeighbours) Direction New%20Neighbour))

(fn CanPlayerEnter
  (params (Player%20Pawn :type Player%20Pawn%20Object%20Reference) (From :type Tile%20Object%20Reference))
  (return true))

(fn ChangeTileType
  (bind _new_tile_type (Variables|Default|GetNew%20Tile%20Type))
  (bind _tile_map (Variables|Default|GetTile%20Map))
  (bind _new_tile_type_2 (Variables|Default|GetNew%20Tile%20Type))
  (if (and (Utilities|IsValidClass _new_tile_type) (!= _new_tile_type (Utilities|GetClass self)))
    (bind _returnvalue (Game|SpawnActorfromClass _new_tile_type_2 (Transformation|GetActorTransform) "AlwaysSpawn" 0 (Variables|Default|GetCoord) (Variables|Default|GetNeighbours) (Variables|Default|GetTile%20Map) _new_tile_type_2 0))
    (bind _keys (Utilities|Map|Keys (Variables|Default|GetNeighbours)))
    (for _array_element _keys
      (Utilities|IsValid (.Value (Utilities|Map|Find (Variables|Default|GetNeighbours) _array_element))
        (:Is%20Valid
          (CallFunction|SetNeighbour (.Value (Utilities|Map|Find (Variables|Default|GetNeighbours) _array_element)) (Variables|/Game/Blueprints/Direction.Direction_C|GetOpposite%20Direction _array_element) _returnvalue)
          (Utilities|Array|Add (Variables|/Game/Blueprints/TileMap.TileMap_C|GetTile _tile_map) _returnvalue)
          (Transformation|AttachActorToActor _returnvalue _tile_map "None" "KeepWorld" "KeepWorld" "KeepWorld" true))))
    (Default|ReplaceTile (Variables|Default|GetTile%20Map) _returnvalue)
    (Actor|DestroyActor)))

(fn CheckifAir
  (if (== "/Game/Blueprints/Air.Air_C" (Utilities|GetClass self))
    (return true)
    (else
      (return false))))

(fn SwapTileCoords
  (params (Tile%20to%20Swap :type Tile%20Object%20Reference))
  (Variables|Default|SetCoordHolder (Variables|Tile_C|GetCoord Tile%20to%20Swap))
  (Variables|Tile_C|SetCoord Tile%20to%20Swap (Variables|Default|GetCoord))
  (Variables|Default|SetCoord (Variables|Default|GetCoordHolder)))

(fn SwapTiles
  (params (String :type String))
  (bind _self self)
  (switch string String
    (:Up
      (Variables|Default|SetTileToSwap (.Value (Utilities|Map|Find (Variables|Default|GetNeighbours) "/Game/Blueprints/Up.Up"))))
    (:Down
      (Variables|Default|SetTileToSwap (.Value (Utilities|Map|Find (Variables|Default|GetNeighbours) "/Game/Blueprints/Down.Down"))))
    (:Left
      (Variables|Default|SetTileToSwap (.Value (Utilities|Map|Find (Variables|Default|GetNeighbours) "/Game/Blueprints/Left.Left"))))
    (:Right
      (Variables|Default|SetTileToSwap (.Value (Utilities|Map|Find (Variables|Default|GetNeighbours) "/Game/Blueprints/Right.Right"))))
    (:Forwards
      (Variables|Default|SetTileToSwap (.Value (Utilities|Map|Find (Variables|Default|GetNeighbours) "/Game/Blueprints/Forwards.Forwards"))))
    (:Back
      (Variables|Default|SetTileToSwap (.Value (Utilities|Map|Find (Variables|Default|GetNeighbours) "/Game/Blueprints/Back.Back")))))
  ;[1 1 1] Swaps Index and Coords between two Tiles
  (Default|SwapTileIndex (Variables|Default|GetTile%20Map) _self (Variables|Default|GetTileToSwap))
  (CallFunction|SwapTileCoords _self (Variables|Default|GetTileToSwap))
  ;[1 1 1] Resets own neighbours and then resets tile to move to neighbours
  (Utilities|Map|Clear (Variables|Tile_C|GetNeighbours (Variables|Default|GetTileToSwap)))
  (CallFunction|FindNeighbours)
  (Utilities|Map|Clear (Variables|Default|GetNeighbours))
  (CallFunction|FindNeighbours self)
  (bind _values (Utilities|Map|Values (Variables|Default|GetNeighbours)))
  (for _array_element _values
    (Utilities|Map|Clear (Variables|Tile_C|GetNeighbours _array_element))
    (CallFunction|FindNeighbours _array_element)
    ;[1 1 1] Resets new tiles neighbours of neighbours, then resets its own neighbours
    (bind _values_2 (Utilities|Map|Values (Variables|Tile_C|GetNeighbours (Variables|Default|GetTileToSwap))))
    (for _array_element_2 _values_2
      (Utilities|Map|Clear (Variables|Tile_C|GetNeighbours _array_element_2))
      (CallFunction|FindNeighbours _array_element_2))))

(fn CheckContainsPlayer
  (if (Utilities|ClassIsChildOf (Utilities|GetClass (Variables|Default|GetPlayerOnTile)) "/Game/Blueprints/PlayerPawn.PlayerPawn_C")
    (return true)
    (else
      (return false))))