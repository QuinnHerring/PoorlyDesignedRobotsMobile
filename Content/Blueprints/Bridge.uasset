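; Movable bridge tile for a grid-based level that can rise, drop or slide horizontally in four directions.
; Each event calls SwapTiles (on completion when dropping) and animates location with a Timeline offset from the starting position.
; A player aboard is carried along with movement locked until the Timeline finishes.
; Otherwise, horizontal moves shift a player on the down-diagonal neighbour one tile onward, or make them fall if that is air.
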(event Custom|Drop%20Bridge
  (bind _returnvalue (Transformation|GetActorLocation))
  (bind _playerontile (Variables|Default|GetPlayerOnTile))
  (bind _playerontile_2 (Variables|Default|GetPlayerOnTile))
  ;[1 1 1] Drop Bridge Down
  (Variables|Default|SetBridgeZ (.z (Transformation|GetActorLocation)))
  (Utilities|IsValid _playerontile
    (:Is%20Valid
      (Variables|/Game/Blueprints/PlayerPawn.PlayerPawn_C|SetcanPlayerMove _playerontile false)
      (Default|DroptoTile (Variables|Default|GetPlayerOnTile) self))
    (:Is%20Not%20Valid
      _))
  (Variables|Default|SetisMoving true)
  (bind _newtrack_0 (Timeline|Dropping PlayFromStart)
    (:Update
      (Transformation|SetActorLocation (Math|Vector|MakeVector (.x _returnvalue) (.y _returnvalue) (- (Variables|Default|GetBridgeZ) _newtrack_0)) false false))
    (:Finished
      (Variables|Default|SetisMoving false)
      (Default|SwapTiles self "Down")
      (Utilities|IsValid _playerontile_2
        (:Is%20Valid
          (Variables|/Game/Blueprints/PlayerPawn.PlayerPawn_C|SetcanPlayerMove _playerontile_2 true))))))

(event Custom|Move%20Bridge%20Right
  (bind _returnvalue (Transformation|GetActorLocation))
  (bind _playerontile (Variables|Default|GetPlayerOnTile))
  (bind _playerontile_2 (Variables|Default|GetPlayerOnTile))
  ;[1 1 1] Move Bridge Right
  (Variables|Default|SetBridgeY (.y (Transformation|GetActorLocation)))
  (Variables|Default|SetDownRightOfBridge (.Value (Utilities|Map|Find (Variables|Default|GetNeighbours) "/Game/Blueprints/DownRight.DownRight")))
  (Default|SwapTiles self "Right")
  (Utilities|IsValid _playerontile
    (:Is%20Valid
      (Variables|/Game/Blueprints/PlayerPawn.PlayerPawn_C|SetcanPlayerMove _playerontile false)
      (Default|MoveRight (Variables|Default|GetPlayerOnTile) self))
    (:Is%20Not%20Valid
      (Utilities|IsValid (Variables|/Game/Blueprints/Tile.Tile_C|GetPlayerOnTile (Variables|Default|GetDownRightOfBridge))
        (:Is%20Valid
          (bind _isair_ (Default|CheckifAir (.Value (Utilities|Map|Find (Variables|/Game/Blueprints/Tile.Tile_C|GetNeighbours (Variables|Default|GetDownRightOfBridge)) "/Game/Blueprints/Right.Right"))))
          (if _isair_
            (Default|Falling (Variables|/Game/Blueprints/Tile.Tile_C|GetPlayerOnTile (Variables|Default|GetDownRightOfBridge)) (.Value (Utilities|Map|Find (Variables|/Game/Blueprints/Tile.Tile_C|GetNeighbours (Variables|Default|GetDownRightOfBridge)) "/Game/Blueprints/Right.Right")))
            (else
              (Default|MovetoTile (Variables|/Game/Blueprints/Tile.Tile_C|GetPlayerOnTile (Variables|Default|GetDownRightOfBridge)) (.Value (Utilities|Map|Find (Variables|/Game/Blueprints/Tile.Tile_C|GetNeighbours (Variables|Default|GetDownRightOfBridge)) "/Game/Blueprints/Right.Right"))))))
        (:Is%20Not%20Valid
          _))))
  (Variables|Default|SetisMoving true)
  (bind _newtrack_0 (Timeline|MoveBridgeRight PlayFromStart)
    (:Update
      (Transformation|SetActorLocation (Math|Vector|MakeVector (.x _returnvalue) (+ _newtrack_0 (Variables|Default|GetBridgeY)) (.z _returnvalue)) false false))
    (:Finished
      (Variables|Default|SetisMoving false)
      (Utilities|IsValid _playerontile_2
        (:Is%20Valid
          (Variables|/Game/Blueprints/PlayerPawn.PlayerPawn_C|SetcanPlayerMove _playerontile_2 true))))))

(event Custom|Move%20Bridge%20Left
  (bind _returnvalue (Transformation|GetActorLocation))
  (bind _playerontile (Variables|Default|GetPlayerOnTile))
  (bind _playerontile_2 (Variables|Default|GetPlayerOnTile))
  ;[1 1 1] Move Bridge Left
  (Variables|Default|SetBridgeY (.y (Transformation|GetActorLocation)))
  (Variables|Default|SetDownLeftOfBridge (.Value (Utilities|Map|Find (Variables|Default|GetNeighbours) "/Game/Blueprints/DownLeft.DownLeft")))
  (Default|SwapTiles self "Left")
  (Utilities|IsValid _playerontile_2
    (:Is%20Valid
      (Variables|/Game/Blueprints/PlayerPawn.PlayerPawn_C|SetcanPlayerMove _playerontile_2 false)
      (Default|MoveLeft (Variables|Default|GetPlayerOnTile) self))
    (:Is%20Not%20Valid
      (Utilities|IsValid (Variables|/Game/Blueprints/Tile.Tile_C|GetPlayerOnTile (Variables|Default|GetDownLeftOfBridge))
        (:Is%20Valid
          (bind _isair_ (Default|CheckifAir (.Value (Utilities|Map|Find (Variables|/Game/Blueprints/Tile.Tile_C|GetNeighbours (Variables|Default|GetDownLeftOfBridge)) "/Game/Blueprints/Left.Left"))))
          (if _isair_
            (Default|Falling (Variables|/Game/Blueprints/Tile.Tile_C|GetPlayerOnTile (Variables|Default|GetDownLeftOfBridge)) (.Value (Utilities|Map|Find (Variables|/Game/Blueprints/Tile.Tile_C|GetNeighbours (Variables|Default|GetDownLeftOfBridge)) "/Game/Blueprints/Left.Left")))
            (else
              (Default|MovetoTile (Variables|/Game/Blueprints/Tile.Tile_C|GetPlayerOnTile (Variables|Default|GetDownLeftOfBridge)) (.Value (Utilities|Map|Find (Variables|/Game/Blueprints/Tile.Tile_C|GetNeighbours (Variables|Default|GetDownLeftOfBridge)) "/Game/Blueprints/Left.Left"))))))
        (:Is%20Not%20Valid
          _))))
  (Variables|Default|SetisMoving true)
  (bind _newtrack_0 (Timeline|MoveBridgeLeft PlayFromStart)
    (:Update
      (Transformation|SetActorLocation (Math|Vector|MakeVector (.x _returnvalue) (- (Variables|Default|GetBridgeY) _newtrack_0) (.z _returnvalue)) false false))
    (:Finished
      (Variables|Default|SetisMoving false)
      (Utilities|IsValid _playerontile
        (:Is%20Valid
          (Variables|/Game/Blueprints/PlayerPawn.PlayerPawn_C|SetcanPlayerMove _playerontile true))))))

(event Custom|Move%20Bridge%20Backwards
  (bind _returnvalue (Transformation|GetActorLocation))
  (bind _playerontile (Variables|Default|GetPlayerOnTile))
  (bind _playerontile_2 (Variables|Default|GetPlayerOnTile))
  ;[1 1 1] Move Bridge Backwards
  (Variables|Default|SetBridgeX (.x (Transformation|GetActorLocation)))
  (Variables|Default|SetDownBackOfBridge (.Value (Utilities|Map|Find (Variables|Default|GetNeighbours) "/Game/Blueprints/DownBack.DownBack")))
  (Default|SwapTiles self "Back")
  (Utilities|IsValid _playerontile
    (:Is%20Valid
      (Variables|/Game/Blueprints/PlayerPawn.PlayerPawn_C|SetcanPlayerMove _playerontile false)
      (Default|MoveBack (Variables|Default|GetPlayerOnTile) self))
    (:Is%20Not%20Valid
      (Utilities|IsValid (Variables|/Game/Blueprints/Tile.Tile_C|GetPlayerOnTile (Variables|Default|GetDownBackOfBridge))
        (:Is%20Valid
          (bind _isair_ (Default|CheckifAir (.Value (Utilities|Map|Find (Variables|/Game/Blueprints/Tile.Tile_C|GetNeighbours (Variables|Default|GetDownBackOfBridge)) "/Game/Blueprints/Back.Back"))))
          (if _isair_
            (Default|Falling (Variables|/Game/Blueprints/Tile.Tile_C|GetPlayerOnTile (Variables|Default|GetDownBackOfBridge)) (.Value (Utilities|Map|Find (Variables|/Game/Blueprints/Tile.Tile_C|GetNeighbours (Variables|Default|GetDownBackOfBridge)) "/Game/Blueprints/Back.Back")))
            (else
              (Default|MovetoTile (Variables|/Game/Blueprints/Tile.Tile_C|GetPlayerOnTile (Variables|Default|GetDownBackOfBridge)) (.Value (Utilities|Map|Find (Variables|/Game/Blueprints/Tile.Tile_C|GetNeighbours (Variables|Default|GetDownBackOfBridge)) "/Game/Blueprints/Back.Back"))))))
        (:Is%20Not%20Valid
          _))))
  (Variables|Default|SetisMoving true)
  (bind _newtrack_0 (Timeline|MoveBridgeBackwards PlayFromStart)
    (:Update
      (Transformation|SetActorLocation (Math|Vector|MakeVector (- (Variables|Default|GetBridgeX) _newtrack_0) (.y _returnvalue) (.z _returnvalue)) false false))
    (:Finished
      (Variables|Default|SetisMoving false)
      (Utilities|IsValid _playerontile_2
        (:Is%20Valid
          (Variables|/Game/Blueprints/PlayerPawn.PlayerPawn_C|SetcanPlayerMove _playerontile_2 true))))))

(event Custom|Raise%20Bridge
  (bind _returnvalue (Transformation|GetActorLocation))
  (bind _playerontile (Variables|Default|GetPlayerOnTile))
  (bind _playerontile_2 (Variables|Default|GetPlayerOnTile))
  ;[1 1 1] Raising Bridge Up
  (Variables|Default|SetBridgeZ (.z (Transformation|GetActorLocation)))
  (Default|SwapTiles self "Up")
  (Utilities|IsValid _playerontile
    (:Is%20Valid
      (Variables|/Game/Blueprints/PlayerPawn.PlayerPawn_C|SetcanPlayerMove _playerontile false)
      (Default|RisetoTile (Variables|Default|GetPlayerOnTile) self))
    (:Is%20Not%20Valid
      _))
  (Variables|Default|SetisMoving true)
  (bind _newtrack_0 (Timeline|Raising PlayFromStart)
    (:Update
      (Transformation|SetActorLocation (Math|Vector|MakeVector (.x _returnvalue) (.y _returnvalue) (+ _newtrack_0 (Variables|Default|GetBridgeZ))) false false))
    (:Finished
      (Variables|Default|SetisMoving false)
      (Utilities|IsValid _playerontile_2
        (:Is%20Valid
          (Variables|/Game/Blueprints/PlayerPawn.PlayerPawn_C|SetcanPlayerMove _playerontile_2 true))))))

(event Custom|Move%20Bridge%20Forwards
  (bind _returnvalue (Transformation|GetActorLocation))
  (bind _playerontile (Variables|Default|GetPlayerOnTile))
  (bind _playerontile_2 (Variables|Default|GetPlayerOnTile))
  ;[1 1 1] Move Bridge Forwards
  (Variables|Default|SetBridgeX (.x (Transformation|GetActorLocation)))
  (Variables|Default|SetDownForwardsOfBridge (.Value (Utilities|Map|Find (Variables|Default|GetNeighbours) "/Game/Blueprints/DownForwards.DownForwards")))
  (Default|SwapTiles self "Forwards")
  (Utilities|IsValid _playerontile_2
    (:Is%20Valid
      (Variables|/Game/Blueprints/PlayerPawn.PlayerPawn_C|SetcanPlayerMove _playerontile_2 false)
      (Default|MoveForwards (Variables|Default|GetPlayerOnTile) self))
    (:Is%20Not%20Valid
      (Utilities|IsValid (Variables|/Game/Blueprints/Tile.Tile_C|GetPlayerOnTile (Variables|Default|GetDownForwardsOfBridge))
        (:Is%20Valid
          (bind _isair_ (Default|CheckifAir (.Value (Utilities|Map|Find (Variables|/Game/Blueprints/Tile.Tile_C|GetNeighbours (Variables|Default|GetDownForwardsOfBridge)) "/Game/Blueprints/Forwards.Forwards"))))
          (if _isair_
            (Default|Falling (Variables|/Game/Blueprints/Tile.Tile_C|GetPlayerOnTile (Variables|Default|GetDownForwardsOfBridge)) (.Value (Utilities|Map|Find (Variables|/Game/Blueprints/Tile.Tile_C|GetNeighbours (Variables|Default|GetDownForwardsOfBridge)) "/Game/Blueprints/Forwards.Forwards")))
            (else
              (Default|MovetoTile (Variables|/Game/Blueprints/Tile.Tile_C|GetPlayerOnTile (Variables|Default|GetDownForwardsOfBridge)) (.Value (Utilities|Map|Find (Variables|/Game/Blueprints/Tile.Tile_C|GetNeighbours (Variables|Default|GetDownForwardsOfBridge)) "/Game/Blueprints/Forwards.Forwards"))))))
        (:Is%20Not%20Valid
          _))))
  (Variables|Default|SetisMoving true)
  (bind _newtrack_0 (Timeline|MoveBridgeForwards PlayFromStart)
    (:Update
      (Transformation|SetActorLocation (Math|Vector|MakeVector (+ _newtrack_0 (Variables|Default|GetBridgeX)) (.y _returnvalue) (.z _returnvalue)) false false))
    (:Finished
      (Variables|Default|SetisMoving false)
      (Utilities|IsValid _playerontile
        (:Is%20Valid
          (Variables|/Game/Blueprints/PlayerPawn.PlayerPawn_C|SetcanPlayerMove _playerontile true))))))

(fn ConstructionScript
  (|CallParentFunction))