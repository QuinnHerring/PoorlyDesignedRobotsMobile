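; Level manager and 3D tile grid for a puzzle game with Orange and Blue pawns on tiles.
; BeginPlay possesses a ControllerPawn and spawns both pawns on their start tiles; ResetMap and coordinate helpers build and index the Floor grid.
; When Tick sees both colours won, it saves fewest moves (Levels 1-2 only), moves the camera and shows a win widget.
; Gamewon unlocks and opens levels through hard-coded level-name chains and PDR_SaveGame.
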(event Custom|Game%20won
  ;[1 1 1] New Level Loading
  (bind _returnvalue (Game|GetCurrentLevelName true))
  (if (Utilities|Enum|Equal(Enum) _returnvalue "Level_1")
    (bind _returnvalue_2 (SaveGame|LoadGamefromSlot "PDR_GameSaveInst"))
    (bind _aspdr_save_game (Utilities|Casting|CastToPDR_SaveGame _returnvalue_2))
    (Variables|/Game/Menus/PDR_SaveGame.PDR_SaveGame_C|SetLevel%202 _aspdr_save_game true)
    (SaveGame|SaveGametoSlot _returnvalue_2 "PDR_GameSaveInst")
    (Game|OpenLevel(byName) "Level_2")
    (elif (Utilities|Enum|Equal(Enum) _returnvalue "Level_2")
      (bind _returnvalue_3 (SaveGame|LoadGamefromSlot "PDR_GameSaveInst"))
      (bind _aspdr_save_game_2 (Utilities|Casting|CastToPDR_SaveGame _returnvalue_3))
      (Variables|/Game/Menus/PDR_SaveGame.PDR_SaveGame_C|SetLevel%203 _aspdr_save_game_2 true)
      (SaveGame|SaveGametoSlot _returnvalue_3 "PDR_GameSaveInst")
      (Game|OpenLevel(byName) "Level_3")
      (elif (Utilities|Enum|Equal(Enum) _returnvalue "Level_3")
        (bind _returnvalue_4 (SaveGame|LoadGamefromSlot "PDR_GameSaveInst"))
        (bind _aspdr_save_game_3 (Utilities|Casting|CastToPDR_SaveGame _returnvalue_4))
        (Variables|/Game/Menus/PDR_SaveGame.PDR_SaveGame_C|SetLevel%204 _aspdr_save_game_3 true)
        (SaveGame|SaveGametoSlot _returnvalue_4 "PDR_GameSaveInst")
        (Game|OpenLevel(byName) "Level_4")
        (elif (Utilities|Enum|Equal(Enum) _returnvalue "Level_4")
          (bind _returnvalue_5 (SaveGame|LoadGamefromSlot "PDR_GameSaveInst"))
          (bind _aspdr_save_game_4 (Utilities|Casting|CastToPDR_SaveGame _returnvalue_5))
          (Variables|/Game/Menus/PDR_SaveGame.PDR_SaveGame_C|SetLevel%205 _aspdr_save_game_4 true)
          (SaveGame|SaveGametoSlot _returnvalue_5 "PDR_GameSaveInst")
          (Game|OpenLevel(byName) "Level_5")
          (elif (Utilities|Enum|Equal(Enum) _returnvalue "Level_5")
            (bind _returnvalue_6 (SaveGame|LoadGamefromSlot "PDR_GameSaveInst"))
            (bind _aspdr_save_game_5 (Utilities|Casting|CastToPDR_SaveGame _returnvalue_6))
            (Variables|/Game/Menus/PDR_SaveGame.PDR_SaveGame_C|SetLevel%206 _aspdr_save_game_5 true)
            (SaveGame|SaveGametoSlot _returnvalue_6 "PDR_GameSaveInst")
            (Game|OpenLevel(byName) "Level_6")
            (elif (Utilities|Enum|Equal(Enum) _returnvalue "Level_6")
              (bind _returnvalue_7 (SaveGame|LoadGamefromSlot "PDR_GameSaveInst"))
              (bind _aspdr_save_game_6 (Utilities|Casting|CastToPDR_SaveGame _returnvalue_7))
              (Variables|/Game/Menus/PDR_SaveGame.PDR_SaveGame_C|SetLevel%206 _aspdr_save_game_6 true)
              (SaveGame|SaveGametoSlot _returnvalue_7 "PDR_GameSaveInst")
              (Game|OpenLevel(byName) "Level_7")
              (elif (Utilities|Enum|Equal(Enum) _returnvalue "Level_7")
                (bind _returnvalue_8 (SaveGame|LoadGamefromSlot "PDR_GameSaveInst"))
                (bind _aspdr_save_game_7 (Utilities|Casting|CastToPDR_SaveGame _returnvalue_8))
                (Variables|/Game/Menus/PDR_SaveGame.PDR_SaveGame_C|SetLevel%207 _aspdr_save_game_7 true)
                (SaveGame|SaveGametoSlot _returnvalue_8 "PDR_GameSaveInst")
                (Game|OpenLevel(byName) "Level_8")
                (elif (Utilities|Enum|Equal(Enum) _returnvalue "Level_8")
                  (bind _returnvalue_9 (SaveGame|LoadGamefromSlot "PDR_GameSaveInst"))
                  (bind _aspdr_save_game_8 (Utilities|Casting|CastToPDR_SaveGame _returnvalue_9))
                  (Variables|/Game/Menus/PDR_SaveGame.PDR_SaveGame_C|SetLevel%208 _aspdr_save_game_8 true)
                  (SaveGame|SaveGametoSlot _returnvalue_9 "PDR_GameSaveInst")
                  (Game|OpenLevel(byName) "Level_9")
                  (elif (Utilities|Enum|Equal(Enum) _returnvalue "Level_9")
                    (bind _returnvalue_10 (SaveGame|LoadGamefromSlot "PDR_GameSaveInst"))
                    (bind _aspdr_save_game_9 (Utilities|Casting|CastToPDR_SaveGame _returnvalue_10))
                    (Variables|/Game/Menus/PDR_SaveGame.PDR_SaveGame_C|SetLevel%209 _aspdr_save_game_9 true)
                    (SaveGame|SaveGametoSlot _returnvalue_10 "PDR_GameSaveInst")
                    (Game|OpenLevel(byName) "Level_10")
                    (elif (Utilities|Enum|Equal(Enum) _returnvalue "Level_10")
                      (bind _returnvalue_11 (SaveGame|LoadGamefromSlot "PDR_GameSaveInst"))
                      (bind _aspdr_save_game_10 (Utilities|Casting|CastToPDR_SaveGame _returnvalue_11))
                      (Variables|/Game/Menus/PDR_SaveGame.PDR_SaveGame_C|SetLevel%2010 _aspdr_save_game_10 true)
                      (SaveGame|SaveGametoSlot _returnvalue_11 "PDR_GameSaveInst")
                      (Game|OpenLevel(byName) "Level_11")
                      (elif (Utilities|Enum|Equal(Enum) _returnvalue "Level_11")
                        (bind _returnvalue_12 (SaveGame|LoadGamefromSlot "PDR_GameSaveInst"))
                        (bind _aspdr_save_game_11 (Utilities|Casting|CastToPDR_SaveGame _returnvalue_12))
                        (Variables|/Game/Menus/PDR_SaveGame.PDR_SaveGame_C|SetLevel%2011 _aspdr_save_game_11 true)
                        (SaveGame|SaveGametoSlot _returnvalue_12 "PDR_GameSaveInst")
                        (Game|OpenLevel(byName) "Level_12")
                        (else
                          (Development|PrintString "Got to the end! What level should we now open?"))))))))))))))

(event Custom|CallFadeIn
  ;[1 1 1] New Level Loading
  (Utilities|FlowControl|DoOnce false
    (:Completed
      (CameraFades|StartCameraFade :self (Game|GetPlayerCameraManager 0) :FromAlpha 1.2 :Duration 4.0 :bHoldWhenFinished true))))

(event Custom|CallFade
  ;[1 1 1] New Level Loading
  (Utilities|FlowControl|DoOnce false
    (:Completed
      (CameraFades|StartCameraFade :self (Game|GetPlayerCameraManager 0) :ToAlpha 1.0 :Duration 2.0 :bHoldWhenFinished (Variables|Default|GetLevel1)))))

(event EventBeginPlay
  (bind _returnvalue (Game|GetPlayerController 0))
  (bind _orange_player_spawn_tile (Variables|Default|GetOrange%20Player%20Spawn%20Tile))
  (bind _blue_player_spawn_tile (Variables|Default|GetBlue%20Player%20Spawn%20Tile))
  (bind _orange_player_direction (Variables|Default|GetOrange%20Player%20Direction))
  (bind _blue_player_direction (Variables|Default|GetBlue%20Player%20Direction))
  (Utilities|FlowControl|Sequence
    (:then_0
      (Audio|PlaySound2D "/Game/Menus/Sounds/Audio_Cues/Level_Music_Cue.Level_Music_Cue" 1.0 1.0 0.0 0 0))
    (:then_1
      (CallFunction|CallFadein)
      (CallFunction|SetNextLevel)
      (bind _returnvalue_2 (Game|SpawnActorfromClass "/Game/Blueprints/ControllerPawn.ControllerPawn_C" (Math|Transform|MakeTransform "0, 0, 0") "Undefined" 0 0))
      (Pawn|Possess _returnvalue _returnvalue_2)
      (Game|Player|SetViewTargetwithBlend _returnvalue (Variables|Default|GetCamera%20Actor) 0.0 "VTBlend_Linear" 0.0 false)
      (bind _returnvalue_3 (Game|SpawnActorfromClass "/Game/Blueprints/PlayerPawn.PlayerPawn_C" (Math|Conversions|ToTransform(Vector) (Transformation|GetActorLocation _orange_player_spawn_tile)) "AlwaysSpawn" 0 0))
      (bind _output_get (Variables|/Game/Blueprints/ControllerPawn.ControllerPawn_C|SetOrangePawn _returnvalue_2 _returnvalue_3))
      (bind _returnvalue_4 (Game|SpawnActorfromClass "/Game/Blueprints/PlayerPawn.PlayerPawn_C" (Math|Conversions|ToTransform(Vector) (Transformation|GetActorLocation _blue_player_spawn_tile)) "AlwaysSpawn" 0 0))
      (bind _output_get_2 (Variables|/Game/Blueprints/ControllerPawn.ControllerPawn_C|SetBluePawn _returnvalue_2 _returnvalue_4))
      (Transformation|SetActorRotation _output_get_2 (Variables|/Game/Blueprints/Direction.Direction_C|GetRotation _blue_player_direction))
      (Transformation|SetActorRotation _output_get (Variables|/Game/Blueprints/Direction.Direction_C|GetRotation _orange_player_direction))
      (Variables|/Game/Blueprints/PlayerPawn.PlayerPawn_C|SetCurrent%20Tile _output_get_2 _blue_player_spawn_tile)
      (Variables|/Game/Blueprints/PlayerPawn.PlayerPawn_C|SetCurrent%20Direction _output_get_2 _blue_player_direction)
      (Variables|/Game/Blueprints/PlayerPawn.PlayerPawn_C|SetCurrent%20Tile _output_get _orange_player_spawn_tile)
      (Variables|/Game/Blueprints/PlayerPawn.PlayerPawn_C|SetCurrent%20Direction _output_get _orange_player_direction)
      (Variables|/Game/Blueprints/Tile.Tile_C|SetPlayerOnTile _blue_player_spawn_tile _output_get_2)
      (Variables|/Game/Blueprints/Tile.Tile_C|SetPlayerOnTile _orange_player_spawn_tile _output_get))))

(event EventTick
  (params (DeltaSeconds :type Float%20%28single-precision%29))
  (bind _camera_actor (Variables|Default|GetCamera%20Actor))
  (bind _rootcomponent (Variables|/Script/Engine.Actor|GetRootComponent _camera_actor))
  (bind _relativerotation (Variables|/Script/Engine.SceneComponent|GetRelativeRotation _rootcomponent))
  (if (and (Variables|Default|GetBlueWon) (Variables|Default|GetOrangeWon))
    (CallFunction|UpdateBestLevelScore)
    (Utilities|FlowControl|Sequence
      (:then_0
        (Utilities|FlowControl|Delay 0.5)
        (CallFunction|CallFade)
        (Variables|Default|SetBlueWon false)
        (Utilities|FlowControl|DoOnce false
          (:Completed
            (if (Variables|Default|GetLevel1)
              (bind _returnvalue (UserInterface|CreateWidget "/Game/Menus/levelWonTest.levelWon_C"))
              (Utilities|FlowControl|DoOnce false
                (:Completed
                  (UserInterface|Animation|PlayAnimation _returnvalue (Variables|/Game/Menus/levelWonTest.levelWon_C|GetShow _returnvalue) 0.0 1 "Forward" 1.0 false)
                  (Utilities|FlowControl|Delay 0.8)
                  (UserInterface|Viewport|AddtoViewport _returnvalue 0)
                  (Utilities|FlowControl|DoOnce false
                    (:Completed
                      (Variables|/Game/Menus/levelWonTest.levelWon_C|Settilemap _returnvalue self)
                      (bind _foundwidgets (Widget|GetAllWidgetsOfClass "/Game/Menus/HUD.HUD_C" true))
                      (UserInterface|Animation|PlayAnimation (Utilities|Array|Get(acopy) _foundwidgets) (Variables|/Game/Menus/HUD.HUD_C|GetFadeOut (Utilities|Array|Get(acopy) _foundwidgets)) 0.0 1 "Forward" 1.0 false)))))
              (else
                (bind _returnvalue_2 (UserInterface|CreateWidget "/Game/Menus/gameWon.gameWon_C"))
                (Utilities|FlowControl|DoOnce false
                  (:Completed
                    (UserInterface|Animation|PlayAnimation _returnvalue_2 (Variables|/Game/Menus/gameWon.gameWon_C|GetfadeIn _returnvalue_2) 0.0 1 "Forward" 1.0 false)
                    (UserInterface|Viewport|AddtoViewport _returnvalue_2 0)
                    (UserInterface|Animation|PlayAnimation _returnvalue_2 (Variables|/Game/Menus/gameWon.gameWon_C|Getwobble _returnvalue_2) 0.0 1001 "Forward" 0.8 false))))))))
      (:then_1
        (Utilities|FlowControl|DoOnce false
          (:Completed
            (Audio|PlaySound2D "/Game/Menus/Sounds/Audio_Cues/Level_Complete_Noise_Cue.Level_Complete_Noise_Cue" 0.5 1.0 0.0 0 0)
            (Components|MoveComponentTo _rootcomponent "-400.000000,-400.000000,680.000000" _relativerotation true true 2.5 false)))))
    (else
      (Utilities|FlowControl|Sequence
        (:then_1
          (Utilities|FlowControl|DoOnce false
            (:Completed
              (Components|MoveComponentTo _rootcomponent "-400.000000,-400.000000,550.000000" _relativerotation true true 2.5 false))))))))

(fn ConstructionScript)

(fn CoordtoIndex
  (params (Coord :type Int%20Vector%20Structure))
  (return (+ (* (.z Coord) (* (Variables|Default|GetWidth) (Variables|Default|GetLength))) (+ (.x Coord) (* (.y Coord) (Variables|Default|GetWidth))))))

(fn ResetMap
  (for _array_element (Variables|Default|GetTile)
    (Utilities|IsValid _array_element
      (:Is%20Valid
        (Actor|DestroyActor _array_element))))
  (Utilities|Array|Clear (Variables|Default|GetTile))
  (for _index (range 0 (- (Variables|Default|GetHeight) 1))
    (for _index_2 (range 0 (- (Variables|Default|GetLength) 1))
      (for _index_3 (range 0 (- (Variables|Default|GetWidth) 1))
        (bind _returnvalue (Game|SpawnActorfromClass "/Game/Blueprints/Floor.Floor_C" (Math|Transform|MakeTransform (Math|Vector|MakeVector (* _index_3 1e+02) (* _index_2 1e+02) (* _index -1e+02)) "0, 0, 0" "1,1,1") "AlwaysSpawn" 0 (Utilities|Struct|MakeIntVector _index_3 _index_2 _index) 0 self 0 0))
        (Utilities|Array|Add (Variables|Default|GetTile) _returnvalue)
        (Transformation|AttachActorToActor _returnvalue self "None" "KeepWorld" "KeepWorld" "KeepWorld" true))))
  (for _array_element_2 (Variables|Default|GetTile)
    (Default|FindNeighbours _array_element_2)))

(fn IsCoordinRange
  (params (Coord :type Int%20Vector%20Structure))
  (return (not (Math|Boolean|ORBoolean (< (.x Coord) 0) (>= (.x Coord) (Variables|Default|GetWidth)) (< (.y Coord) 0) (>= (.y Coord) (Variables|Default|GetLength)) (< (.z Coord) 0) (>= (.z Coord) (Variables|Default|GetHeight))))))

(fn GetTileatCoord
  (params (Coord :type Int%20Vector%20Structure))
  (return (Utilities|Array|Get(acopy) (Variables|Default|GetTile) (CallFunction|CoordtoIndex (Utilities|Struct|MakeIntVector (.x Coord) (.y Coord) (.z Coord))))))

(fn ReplaceTile
  (params (New%20Tile :type Tile%20Object%20Reference))
  (Utilities|Array|SetArrayElem (Variables|Default|GetTile) (CallFunction|CoordtoIndex (Variables|/Game/Blueprints/Tile.Tile_C|GetCoord New%20Tile)) New%20Tile))

(fn SwapTileIndex
  (params (Tile%20A :type Tile%20Object%20Reference) (Tile%20B :type Tile%20Object%20Reference))
  (Utilities|Array|SetArrayElem (Variables|Default|GetTile) (CallFunction|CoordtoIndex (Variables|/Game/Blueprints/Tile.Tile_C|GetCoord Tile%20A)) Tile%20B)
  (Utilities|Array|SetArrayElem (Variables|Default|GetTile) (CallFunction|CoordtoIndex (Variables|/Game/Blueprints/Tile.Tile_C|GetCoord Tile%20B)) Tile%20A))

(fn SetNextLevel
  (bind _returnvalue (Game|GetCurrentLevelName true))
  (if (Utilities|Enum|Equal(Enum) _returnvalue "Level_1")
    (Variables|Default|SetLevel%20Name "LEVEL 2")
    (else
      (bind _returnvalue_2 (Game|GetCurrentLevelName true))
      (if (Utilities|Enum|Equal(Enum) _returnvalue_2 "Level_2")
        (Variables|Default|SetLevel%20Name "LEVEL 3")
        (else
          (bind _returnvalue_3 (Game|GetCurrentLevelName true))
          (if (Utilities|Enum|Equal(Enum) _returnvalue_3 "Level_3")
            (Variables|Default|SetLevel%20Name "LEVEL 4")
            (else
              (bind _returnvalue_4 (Game|GetCurrentLevelName true))
              (if (Utilities|Enum|Equal(Enum) _returnvalue_4 "Level_4")
                (Variables|Default|SetLevel%20Name "LEVEL 5")
                (else
                  (bind _returnvalue_5 (Game|GetCurrentLevelName true))
                  (if (Utilities|Enum|Equal(Enum) _returnvalue_5 "Level_4")
                    (Variables|Default|SetLevel%20Name "LEVEL 5")
                    (else
                      (bind _returnvalue_6 (Game|GetCurrentLevelName true))
                      (if (Utilities|Enum|Equal(Enum) _returnvalue_6 "Level_5")
                        (Variables|Default|SetLevel%20Name "LEVEL 6")
                        (else
                          (bind _returnvalue_7 (Game|GetCurrentLevelName true))
                          (if (Utilities|Enum|Equal(Enum) _returnvalue_7 "Level_6")
                            (Variables|Default|SetLevel%20Name "LEVEL 7")
                            (else
                              (bind _returnvalue_8 (Game|GetCurrentLevelName true))
                              (if (Utilities|Enum|Equal(Enum) _returnvalue_8 "Level_7")
                                (Variables|Default|SetLevel%20Name "LEVEL 8")
                                (else
                                  (bind _returnvalue_9 (Game|GetCurrentLevelName true))
                                  (if (Utilities|Enum|Equal(Enum) _returnvalue_9 "Level_8")
                                    (Variables|Default|SetLevel%20Name "LEVEL 9")
                                    (else
                                      (bind _returnvalue_10 (Game|GetCurrentLevelName true))
                                      (if (Utilities|Enum|Equal(Enum) _returnvalue_10 "Level_9")
                                        (Variables|Default|SetLevel%20Name "LEVEL 10")
                                        (else
                                          (bind _returnvalue_11 (Game|GetCurrentLevelName true))
                                          (if (Utilities|Enum|Equal(Enum) _returnvalue_11 "Level_10")
                                            (Variables|Default|SetLevel%20Name "LEVEL 11")))))))))))))))))))))))

(fn UpdateBestLevelScore
  (bind _returnvalue (SaveGame|LoadGamefromSlot "PDR_GameSaveInst"))
  (bind _aspdr_save_game (Utilities|Casting|CastToPDR_SaveGame _returnvalue))
  (Variables|Default|SetPDR_SaveGameInst _aspdr_save_game)
  (bind _returnvalue_2 (Game|GetCurrentLevelName true))
  (if (Utilities|Enum|Equal(Enum) _returnvalue_2 "Level_1")
    (bind _new_high_score (CallFunction|GetNewBestLevelScore (Variables|/Game/Menus/PDR_SaveGame.PDR_SaveGame_C|GetLevel%201%20Moves (Variables|Default|GetPDR_SaveGameInst)) (Variables|/Game/Menus/PDR_SaveGame.PDR_SaveGame_C|GetCurrent%20Moves%20Taken (Variables|Default|GetPDR_SaveGameInst))))
    (Variables|/Game/Menus/PDR_SaveGame.PDR_SaveGame_C|SetLevel%201%20Moves (Variables|Default|GetPDR_SaveGameInst) _new_high_score)
    (SaveGame|SaveGametoSlot (Variables|Default|GetPDR_SaveGameInst) (Variables|/Game/Menus/PDR_SaveGame.PDR_SaveGame_C|GetSave%20Slot%20Name (Variables|Default|GetPDR_SaveGameInst)))
    (elif (Utilities|Enum|Equal(Enum) _returnvalue_2 "Level_2")
      (bind _new_high_score_2 (CallFunction|GetNewBestLevelScore (Variables|/Game/Menus/PDR_SaveGame.PDR_SaveGame_C|GetLevel%202%20Moves (Variables|Default|GetPDR_SaveGameInst)) (Variables|/Game/Menus/PDR_SaveGame.PDR_SaveGame_C|GetCurrent%20Moves%20Taken (Variables|Default|GetPDR_SaveGameInst))))
      (Variables|/Game/Menus/PDR_SaveGame.PDR_SaveGame_C|SetLevel%202%20Moves (Variables|Default|GetPDR_SaveGameInst) _new_high_score_2)
      (SaveGame|SaveGametoSlot (Variables|Default|GetPDR_SaveGameInst) (Variables|/Game/Menus/PDR_SaveGame.PDR_SaveGame_C|GetSave%20Slot%20Name (Variables|Default|GetPDR_SaveGameInst)))
      (elif (not (Utilities|Enum|Equal(Enum) _returnvalue_2 "Level_3"))
        (if (not (Utilities|Enum|Equal(Enum) _returnvalue_2 "Level_4"))
          (if (not (Utilities|Enum|Equal(Enum) _returnvalue_2 "Level_5"))
            (if (not (Utilities|Enum|Equal(Enum) _returnvalue_2 "Level_6"))
              (if (not (Utilities|Enum|Equal(Enum) _returnvalue_2 "Level_7"))
                (if (not (Utilities|Enum|Equal(Enum) _returnvalue_2 "Level_8"))
                  (if (not (Utilities|Enum|Equal(Enum) _returnvalue_2 "Level_9"))
                    (if (not (Utilities|Enum|Equal(Enum) _returnvalue_2 "Level_10"))
                      (if (Utilities|Enum|Equal(Enum) _returnvalue_2 "Level_11")
                        _))))))))))))

(fn GetNewBestLevelScore
  (params (Current%20High%20Score :type Integer) (Proposed%20high%20Score :type Integer))
  (if (== Current%20High%20Score 0)
    _
    (elif (< Proposed%20high%20Score Current%20High%20Score)
      _
      (else
        (return Current%20High%20Score))))
  (return Proposed%20high%20Score))