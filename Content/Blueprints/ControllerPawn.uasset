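; Player controller pawn for a tile-based two-robot puzzle: left/right moves the orange pawn, up/down moves the blue one.
; Tick repeats held moves, locked by a delay that MoveAPlayer returns, and writes the move count to the save game.
; MoveAPlayer checks neighbour tiles via direction-array offsets, recursing to push or carry the other pawn and calling FallAPlayer for drops.
; It also creates the HUD and opens the pause menu on Escape.
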(event EventTick
  (params (DeltaSeconds :type Float%20%28single-precision%29))
  (bind _bluepawn (Variables|Default|GetBluePawn))
  (bind _orangepawn (Variables|Default|GetOrangePawn))
  (bind _current_tile (Variables|/Game/Blueprints/PlayerPawn.PlayerPawn_C|GetCurrent%20Tile _orangepawn))
  (bind _current_tile_2 (Variables|/Game/Blueprints/PlayerPawn.PlayerPawn_C|GetCurrent%20Tile _bluepawn))
  (bind _neighbours (Variables|/Game/Blueprints/Tile.Tile_C|GetNeighbours _current_tile))
  (bind _neighbours_2 (Variables|/Game/Blueprints/Tile.Tile_C|GetNeighbours _current_tile_2))
  (bind _value (Utilities|Map|Find _neighbours_2 "/Game/Blueprints/Down.Down"))
  (bind _value_2 (Utilities|Map|Find _neighbours "/Game/Blueprints/Down.Down"))
  (if (Variables|Default|GetKeyHeld)
    (switch string (Variables|Default|GetKeyType)
      (:Left
        (if (Variables|Default|GetCanPlayerMove)
          (if (Variables|/Game/Blueprints/PlayerPawn.PlayerPawn_C|GetisOnTop _orangepawn)
            (Variables|/Game/Blueprints/PlayerPawn.PlayerPawn_C|SetisOnTop _orangepawn false)
            (else
              (bind _contains_player (Default|CheckContainsPlayer _value_2))
              (if _contains_player
                (Variables|/Game/Blueprints/PlayerPawn.PlayerPawn_C|SetisOnTop _orangepawn true)
                (else
                  (Variables|/Game/Blueprints/PlayerPawn.PlayerPawn_C|SetisOnTop _orangepawn false)))))
          (bind _wait_length (CallFunction|MoveAPlayer "/Game/Blueprints/Left.Left" _orangepawn))
          (Variables|Default|SetWait _wait_length)
          (Variables|Default|SetCanPlayerMove false :!label _label)
          (Audio|PlaySound2D "/Game/Menus/Sounds/Wavs/Robot_Movement.Robot_Movement" 1.0 1.0 0.0 0 0)
          (Utilities|FlowControl|Delay (Variables|Default|GetWait))
          (Variables|Default|SetCanPlayerMove true)
          (bind _output_get (Variables|Default|SetMovesTaken (+ (Variables|Default|GetMovesTaken) 1) :!label _label_2))
          (CallFunction|UpdateMovesTaken _output_get)))
      (:Right
        (if (Variables|Default|GetCanPlayerMove)
          (if (Variables|/Game/Blueprints/PlayerPawn.PlayerPawn_C|GetisOnTop _orangepawn)
            (Variables|/Game/Blueprints/PlayerPawn.PlayerPawn_C|SetisOnTop _orangepawn false)
            (else
              (bind _contains_player_2 (Default|CheckContainsPlayer _value_2))
              (if _contains_player_2
                (Variables|/Game/Blueprints/PlayerPawn.PlayerPawn_C|SetisOnTop _orangepawn true)
                (else
                  (Variables|/Game/Blueprints/PlayerPawn.PlayerPawn_C|SetisOnTop _orangepawn false)))))
          (bind _wait_length_2 (CallFunction|MoveAPlayer "/Game/Blueprints/Right.Right" _orangepawn))
          (Variables|Default|SetWait _wait_length_2)
          (goto _label)))
      (:Up
        (if (Variables|Default|GetCanPlayerMove)
          (if (Variables|/Game/Blueprints/PlayerPawn.PlayerPawn_C|GetisOnTop _bluepawn)
            (Variables|/Game/Blueprints/PlayerPawn.PlayerPawn_C|SetisOnTop _bluepawn false)
            (else
              (bind _contains_player_3 (Default|CheckContainsPlayer _value))
              (if _contains_player_3
                (Variables|/Game/Blueprints/PlayerPawn.PlayerPawn_C|SetisOnTop _bluepawn true)
                (else
                  (Variables|/Game/Blueprints/PlayerPawn.PlayerPawn_C|SetisOnTop _bluepawn false)))))
          (bind _wait_length_3 (CallFunction|MoveAPlayer "/Game/Blueprints/Forwards.Forwards" _bluepawn))
          (Variables|Default|SetWait _wait_length_3)
          (Variables|Default|SetCanPlayerMove false :!label _label_3)
          (Audio|PlaySound2D "/Game/Menus/Sounds/Audio_Cues/Robot_Movement_Cue.Robot_Movement_Cue" 1.0 1.0 0.0 0 0)
          (Utilities|FlowControl|Delay (Variables|Default|GetWait))
          (Variables|Default|SetCanPlayerMove true)
          (goto _label_2)))
      (:Down
        (if (Variables|Default|GetCanPlayerMove)
          (if (Variables|/Game/Blueprints/PlayerPawn.PlayerPawn_C|GetisOnTop _bluepawn)
            (Variables|/Game/Blueprints/PlayerPawn.PlayerPawn_C|SetisOnTop _bluepawn false)
            (else
              (bind _contains_player_4 (Default|CheckContainsPlayer _value))
              (if _contains_player_4
                (Variables|/Game/Blueprints/PlayerPawn.PlayerPawn_C|SetisOnTop _bluepawn true)
                (else
                  (Variables|/Game/Blueprints/PlayerPawn.PlayerPawn_C|SetisOnTop _bluepawn false)))))
          (bind _wait_length_4 (CallFunction|MoveAPlayer "/Game/Blueprints/Back.Back" _bluepawn))
          (Variables|Default|SetWait _wait_length_4)
          (goto _label_3))))))

(event EventBeginPlay
  (bind _returnvalue (UserInterface|CreateWidget "/Game/Menus/HUD.HUD_C"))
  (bind _output_get (Variables|Default|SetHUD%20Reference _returnvalue))
  (UserInterface|Viewport|AddtoViewport _output_get 0)
  (CallFunction|UpdateMovesTaken))

(event Input|ActionEvents|InputActionMoveDown
  (params (Key :type Key%20Structure :default "None"))
  (:Pressed
    (Variables|Default|SetKeyHeld true)
    (Variables|Default|SetKeyType "Down"))
  (:Released
    (Variables|Default|SetKeyHeld false)))

(event Input|ActionEvents|InputActionMoveLeft
  (params (Key :type Key%20Structure :default "None"))
  (:Pressed
    (Variables|Default|SetKeyHeld true)
    (Variables|Default|SetKeyType "Left"))
  (:Released
    (Variables|Default|SetKeyHeld false)))

(event Input|ActionEvents|InputActionMoveRight
  (params (Key :type Key%20Structure :default "None"))
  (:Pressed
    (Variables|Default|SetKeyHeld true)
    (Variables|Default|SetKeyType "Right"))
  (:Released
    (Variables|Default|SetKeyHeld false)))

(event Input|ActionEvents|InputActionMoveUp
  (params (Key :type Key%20Structure :default "None"))
  (:Pressed
    (Variables|Default|SetKeyHeld true)
    (Variables|Default|SetKeyType "Up"))
  (:Released
    (Variables|Default|SetKeyHeld false)))

(event Input|KeyboardEvents|Escape
  (params (Key :type Key%20Structure :default "None"))
  ;[1 1 1] Open Pause Menu
  (:Pressed
    (CameraFades|StartCameraFade :self (Game|GetPlayerCameraManager 0) :ToAlpha 0.9 :Duration 1e-05 :bHoldWhenFinished true)
    (bind _returnvalue (UserInterface|CreateWidget "/Game/Menus/Pause_Widget.Pause_Widget_C"))
    (Utilities|FlowControl|Delay 0.0001)
    (UserInterface|Viewport|AddtoViewport _returnvalue 0)
    (Variables|/Script/Engine.PlayerController|SetbShowMouseCursor (Game|GetPlayerController 0) true)))

(fn ConstructionScript
  (Variables|Default|SetCanPlayerMove true))

(fn MoveAPlayer
  (params (Move%20Direction :type Direction%20Object%20Reference) (Player%20To%20Move :type Player%20Pawn%20Object%20Reference))
  (bind _array (Utilities|Array|MakeArray "/Game/Blueprints/Forwards.Forwards" "/Game/Blueprints/Back.Back" "/Game/Blueprints/Left.Left" "/Game/Blueprints/Right.Right" "/Game/Blueprints/upForwards.UpForwards" "/Game/Blueprints/UpBack.UpBack" "/Game/Blueprints/UpLeft.UpLeft" "/Game/Blueprints/UpRight.UpRight" "/Game/Blueprints/DownForwards.DownForwards" "/Game/Blueprints/DownBack.DownBack" "/Game/Blueprints/DownLeft.DownLeft" "/Game/Blueprints/DownRight.DownRight" "/Game/Blueprints/Up.Up" "/Game/Blueprints/Down.Down"))
  (bind _current_tile (Variables|/Game/Blueprints/PlayerPawn.PlayerPawn_C|GetCurrent%20Tile Player%20To%20Move))
  (bind _returnvalue (Utilities|Array|FindItem _array Move%20Direction))
  (bind _neighbours (Variables|/Game/Blueprints/Tile.Tile_C|GetNeighbours _current_tile))
  (bind _value (Utilities|Map|Find _neighbours "/Game/Blueprints/Up.Up"))
  (bind _value_2 (Utilities|Map|Find _neighbours Move%20Direction))
  (bind _returnvalue_2 (+ _returnvalue 4))
  (bind _returnvalue_3 (+ _returnvalue 8))
  (bind _output (Utilities|Array|Get(acopy) _array _returnvalue_2))
  (bind _output_2 (Utilities|Array|Get(acopy) _array _returnvalue_3))
  (bind _value_3 (Utilities|Map|Find _neighbours _output))
  (bind _value_4 (Utilities|Map|Find _neighbours _output_2))
  ;[1 1 1] MASTER
  (if (or (Variables|Default|GetOrangeNotWon) (Variables|Default|GetBlueNotWon))
    (Utilities|IsValid (Variables|/Game/Blueprints/PlayerPawn.PlayerPawn_C|GetTarget%20Tile Player%20To%20Move)
      (:Is%20Valid
        _)
      (:Is%20Not%20Valid
        (Utilities|IsValid _value_3
          (:Is%20Valid
            (bind _isair_ (Default|CheckifAir _value_3))
            (if _isair_
              (Utilities|IsValid _value_2
                (:Is%20Valid
                  (bind _isair__2 (Default|CheckifAir _value_2))
                  (if _isair__2
                    (if (Variables|/Game/Blueprints/PlayerPawn.PlayerPawn_C|GetisOnTop Player%20To%20Move)
                      (if (stale _contains_player_4) :!label _label
                        (bind _moveisvalid (CallFunction|MoveAPlayer Move%20Direction (Variables|/Game/Blueprints/Tile.Tile_C|GetPlayerOnTile _value_2)))
                        (if _moveisvalid
                          (Default|MovetoTile Player%20To%20Move _value_2 :!label _label_2)
                          (bind _contains_player (Default|CheckContainsPlayer _value))
                          (if _contains_player
                            (bind _output_player (CallFunction|GetOtherPlayer Player%20To%20Move))
                            (bind _moveisvalid_2 (CallFunction|MoveAPlayer Move%20Direction _output_player))
                            (if _moveisvalid_2
                              _
                              (else
                                (Variables|/Game/Blueprints/PlayerPawn.PlayerPawn_C|SetisOnTop _output_player false)
                                (bind _full_falling_ (CallFunction|FallAPlayer _output_player (Variables|/Game/Blueprints/PlayerPawn.PlayerPawn_C|GetCurrent%20Tile _output_player) (.Value (Utilities|Map|Find (Variables|/Game/Blueprints/Tile.Tile_C|GetNeighbours (Variables|/Game/Blueprints/PlayerPawn.PlayerPawn_C|GetCurrent%20Tile _output_player)) "/Game/Blueprints/Down.Down")) true true))
                                (if _full_falling_
                                  (Variables|Default|SetReturn%20Length 1.2)
                                  (else
                                    (Variables|Default|SetReturn%20Length 0.7)))))
                            (else
                              (bind _contains_player_2 (Default|CheckContainsPlayer _value_4 :!label _label_3))
                              (if _contains_player_2
                                (Variables|/Game/Blueprints/PlayerPawn.PlayerPawn_C|SetisOnTop Player%20To%20Move true))))
                          (return true (Variables|Default|GetReturn%20Length))
                          (else
                            _))
                        (else
                          (Variables|Default|SetReturn%20Length 0.5)
                          (goto _label_2)))
                      (else
                        (bind _full_falling__2 (CallFunction|FallAPlayer Player%20To%20Move _value_2 _value_4 false false))
                        (if _full_falling__2
                          (Variables|Default|SetReturn%20Length 1.2)
                          (else
                            (Variables|Default|SetReturn%20Length 0.7)))
                        (bind _contains_player_3 (Default|CheckContainsPlayer _value))
                        (if _contains_player_3
                          (bind _output_player_2 (CallFunction|GetOtherPlayer Player%20To%20Move))
                          (CallFunction|FallAPlayer _output_player_2 (.Value (Utilities|Map|Find (Variables|/Game/Blueprints/Tile.Tile_C|GetNeighbours _value_2) "/Game/Blueprints/Up.Up")) (.Value (Utilities|Map|Find (Variables|/Game/Blueprints/Tile.Tile_C|GetNeighbours _value_4) "/Game/Blueprints/Up.Up")) true _full_falling__2)
                          (return true (Variables|Default|GetReturn%20Length))
                          (else
                            (goto _label_3)))))
                    (else
                      (bind _contains_player_4 (Default|CheckContainsPlayer _value_2))
                      (goto _label))))
                (:Is%20Not%20Valid
                  _))))
          (:Is%20Not%20Valid
            _)))))
  (return false 0.0))

(fn FallAPlayer
  (params (Player%20To%20Move :type Player%20Pawn%20Object%20Reference) (Side%20Tile :type Tile%20Object%20Reference) (Down%20Tile :type Tile%20Object%20Reference) (Force%20Fall :type Boolean) (Force%20Fall%20Type :type Boolean))
  (bind _neighbours (Variables|/Game/Blueprints/Tile.Tile_C|GetNeighbours Side%20Tile))
  (bind _value (Utilities|Map|Find _neighbours "/Game/Blueprints/Down.Down"))
  (if Force%20Fall
    (if Force%20Fall%20Type
      (bind _isair_ (Default|CheckifAir _value))
      (if _isair_
        (Default|Falling Player%20To%20Move Down%20Tile)
        (return true)
        (else
          _)))
    (Default|FalltoTile Player%20To%20Move Down%20Tile)
    (else
      (bind _isair__2 (Default|CheckifAir _value))
      (if _isair__2
        (Default|Falling Player%20To%20Move Down%20Tile)
        (return true)
        (else
          (bind _contains_player (Default|CheckContainsPlayer _value))
          (if _contains_player
            (Default|MovetoTile Player%20To%20Move Side%20Tile)
            (else
              (Default|FalltoTile Player%20To%20Move Down%20Tile)))))))
  (return false))

(fn GetOtherPlayer
  (params (Input%20Player :type Player%20Pawn%20Object%20Reference))
  (bind _bluepawn (Variables|Default|GetBluePawn))
  (if (== Input%20Player _bluepawn)
    (return (Variables|Default|GetOrangePawn))
    (else
      (return _bluepawn))))

(fn UpdateMovesTaken
  (params (New%20Moves%20Taken :type Integer))
  (bind _returnvalue (SaveGame|LoadGamefromSlot "PDR_GameSaveInst"))
  (bind _aspdr_save_game (Utilities|Casting|CastToPDR_SaveGame _returnvalue))
  (Variables|/Game/Menus/PDR_SaveGame.PDR_SaveGame_C|SetCurrent%20Moves%20Taken _aspdr_save_game New%20Moves%20Taken)
  (SaveGame|SaveGametoSlot _aspdr_save_game (Variables|/Game/Menus/PDR_SaveGame.PDR_SaveGame_C|GetSave%20Slot%20Name _aspdr_save_game)))