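; BP_Button is a pressure-style button that switches a linked object on and off through overlaps with its Trigger.
; The first overlap sets Pressed, and an end overlap clears it only when fewer than two actors remain in the trigger's overlap list.
; Each of these updates swaps the Button material to match the state and passes Pressed to ObjectToAffect via TurnSwitchMessage.
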(event OnComponentBeginOverlap(Trigger)
  (params (OverlappedComponent :type Primitive%20Component%20Object%20Reference) (OtherActor :type Actor%20Object%20Reference) (OtherComp :type Primitive%20Component%20Object%20Reference) (OtherBodyIndex :type Integer) (bFromSweep :type Boolean) (SweepResult :type Hit%20Result%20Structure%20%28by%20ref%29))
  (if (not (Variables|Default|GetPressed))
    (Variables|Default|SetPressed true)
    (if (Variables|Default|GetPressed)
      (Rendering|Material|SetMaterial (Variables|Default|GetButton) 0 "/Engine/EditorMaterials/WidgetMaterial_Y.WidgetMaterial_Y")
      (else
        (Rendering|Material|SetMaterial (Variables|Default|GetButton) 0 "/Engine/EditorMaterials/WidgetMaterial_X.WidgetMaterial_X")))
    (Class|BPTurnSwitch|TurnSwitch(Message) (Variables|Default|GetObjectToAffect) (Variables|Default|GetPressed))))

(event OnComponentEndOverlap(Trigger)
  (params (OverlappedComponent :type Primitive%20Component%20Object%20Reference) (OtherActor :type Actor%20Object%20Reference) (OtherComp :type Primitive%20Component%20Object%20Reference) (OtherBodyIndex :type Integer))
  (if (not (Utilities|Array|IsValidIndex (Collision|GetOverlappingActors (Variables|Default|GetTrigger) 0 :!class /Script/Engine.PrimitiveComponent) 1))
    (Variables|Default|SetPressed false)
    (if (Variables|Default|GetPressed)
      (Rendering|Material|SetMaterial (Variables|Default|GetButton) 0 "/Engine/EditorMaterials/WidgetMaterial_Y.WidgetMaterial_Y")
      (else
        (Rendering|Material|SetMaterial (Variables|Default|GetButton) 0 "/Engine/EditorMaterials/WidgetMaterial_X.WidgetMaterial_X")))
    (Class|BPTurnSwitch|TurnSwitch(Message) (Variables|Default|GetObjectToAffect) (Variables|Default|GetPressed))))

(fn ConstructionScript
  (|CallParentFunction))