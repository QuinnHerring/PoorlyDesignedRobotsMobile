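; Player pawn for a tile-based game with orange and blue pawns, handling timeline-animated movement between tiles.
; Move and fall-to-tile events check CanPlayerEnter and bridge motion, lerp across (falls then drop), and update tile occupancy on finish.
; Separate events offset the pawn along one axis for rises, drops and directional moves, while Falling prints "Game Over".
; SwitchPlayers teleport-swaps both pawns and their CurrentTile references via the ControllerPawn.
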(event Custom|Fall%20to%20Tile
  (params (Tile%20to%20Fall%20to :type Tile%20Object%20Reference))
  ;[1 1 1] MASTER
  (if (Variables|Default|GetcanPlayerMove)
    (Utilities|IsValid Tile%20to%20Fall%20to
      (:Is%20Valid
        (if (Default|CanPlayerEnter Tile%20to%20Fall%20to self (Variables|Default|GetCurrent%20Tile))
          (bind _bridgemoving_ (Default|CheckifBridgeMoving Tile%20to%20Fall%20to))
          (if (not _bridgemoving_)
            (Variables|Default|SetTarget%20Tile Tile%20to%20Fall%20to)
            (bind _move_progress (Timeline|MoveToTile2 PlayFromStart)
              (:Update
                (Transformation|SetActorLocation (Math|Vector|Lerp(Vector) (Math|Vector|MakeVector (.x (Transformation|GetActorLocation (Variables|Default|GetCurrent%20Tile))) (.y (Transformation|GetActorLocation (Variables|Default|GetCurrent%20Tile))) (.z (Transformation|GetActorLocation (Variables|Default|GetCurrent%20Tile)))) (Math|Vector|MakeVector (.x (Transformation|GetActorLocation (Variables|Default|GetTarget%20Tile))) (.y (Transformation|GetActorLocation (Variables|Default|GetTarget%20Tile))) (.z (Transformation|GetActorLocation (Variables|Default|GetCurrent%20Tile)))) _move_progress) false false))
              (:Finished
                (bind _fall_progress (Timeline|DropToTile PlayFromStart)
                  (:Update
                    (Transformation|SetActorLocation (Math|Vector|Lerp(Vector) (Math|Vector|MakeVector (.x (Transformation|GetActorLocation (Variables|Default|GetTarget%20Tile))) (.y (Transformation|GetActorLocation (Variables|Default|GetTarget%20Tile))) (.z (Transformation|GetActorLocation (Variables|Default|GetCurrent%20Tile)))) (Math|Vector|MakeVector (.x (Transformation|GetActorLocation (Variables|Default|GetTarget%20Tile))) (.y (Transformation|GetActorLocation (Variables|Default|GetTarget%20Tile))) (.z (Transformation|GetActorLocation (Variables|Default|GetTarget%20Tile)))) _fall_progress) false false))
                  (:Finished
                    (Variables|/Game/Blueprints/Tile.Tile_C|SetPlayerOnTile (Variables|Default|GetTarget%20Tile) self)
                    (Variables|/Game/Blueprints/Tile.Tile_C|SetPlayerOnTile (Variables|Default|GetCurrent%20Tile) 0)
                    (Variables|Default|SetCurrent%20Tile (Variables|Default|GetTarget%20Tile))
                    (Variables|Default|SetTarget%20Tile 0)))))))))))

(event Custom|Move%20to%20Tile
  (params (Tile%20to%20Move%20to :type Tile%20Object%20Reference))
  ;[1 1 1] MASTER
  (if (Variables|Default|GetcanPlayerMove)
    (Utilities|IsValid Tile%20to%20Move%20to
      (:Is%20Valid
        (if (Default|CanPlayerEnter Tile%20to%20Move%20to self (Variables|Default|GetCurrent%20Tile))
          (bind _bridgemoving_ (Default|CheckifBridgeMoving Tile%20to%20Move%20to))
          (if (not _bridgemoving_)
            (Variables|Default|SetTarget%20Tile Tile%20to%20Move%20to)
            (bind _move_progress (Timeline|MoveToTile PlayFromStart)
              (:Update
                (Transformation|SetActorLocation (Math|Vector|Lerp(Vector) (Transformation|GetActorLocation (Variables|Default|GetCurrent%20Tile)) (Transformation|GetActorLocation (Variables|Default|GetTarget%20Tile)) _move_progress) false false))
              (:Finished
                (Variables|/Game/Blueprints/Tile.Tile_C|SetPlayerOnTile (Variables|Default|GetTarget%20Tile) self)
                (Variables|/Game/Blueprints/Tile.Tile_C|SetPlayerOnTile (Variables|Default|GetCurrent%20Tile) 0)
                (Variables|Default|SetCurrent%20Tile (Variables|Default|GetTarget%20Tile))
                (Variables|Default|SetTarget%20Tile 0)))))))))

(event Custom|Move%20Left
  (params (Tile%20to%20Move%20to :type Tile%20Object%20Reference))
  (bind _returnvalue (Transformation|GetActorLocation Tile%20to%20Move%20to))
  ;[1 1 1] MASTER
  (Variables|Default|SetCurrentY (.y (Transformation|GetActorLocation self)))
  (bind _movingtoleft (Timeline|MoveToLeft_TL PlayFromStart)
    (:Update
      (Transformation|SetActorLocation (Math|Vector|MakeVector (.x _returnvalue) (+ _movingtoleft (Variables|Default|GetCurrentY)) (.z _returnvalue)) false false))))

(event Custom|Rise%20to%20Tile
  (params (Tile%20to%20Rise%20To :type Tile%20Object%20Reference))
  (bind _returnvalue (Transformation|GetActorLocation Tile%20to%20Rise%20To))
  ;[1 1 1] MASTER
  (Variables|Default|SetCurrentZ (.z (Transformation|GetActorLocation self)))
  (bind _newtrack_0 (Timeline|RiseToTile PlayFromStart)
    (:Update
      (Transformation|SetActorLocation (Math|Vector|MakeVector (.x _returnvalue) (.y _returnvalue) (+ _newtrack_0 (Variables|Default|GetCurrentZ))) false false))))

(event Custom|Falling
  (params (Tile%20To%20Fall%20To :type Tile%20Object%20Reference))
  (bind _current_tile (Variables|Default|GetCurrent%20Tile))
  (bind _returnvalue (Transformation|GetActorLocation _current_tile))
  ;[1 1 1] MASTER
  (Variables|Default|SetTarget%20Tile Tile%20To%20Fall%20To)
  (bind _moving (Timeline|Timeline_5 PlayFromStart)
    (:Update
      (Transformation|SetActorLocation (Math|Vector|Lerp(Vector) (Math|Vector|MakeVector (.x _returnvalue) (.y _returnvalue) (.z _returnvalue)) (Math|Vector|MakeVector (.x (Transformation|GetActorLocation (Variables|Default|GetTarget%20Tile))) (.y (Transformation|GetActorLocation (Variables|Default|GetTarget%20Tile))) (.z _returnvalue)) _moving) false false))
    (:Finished
      (bind _falling (Timeline|Timeline_4 PlayFromStart)
        (:Update
          (Transformation|SetActorLocation (Math|Vector|MakeVector (.x (Transformation|GetActorLocation (Variables|Default|GetTarget%20Tile))) (.y (Transformation|GetActorLocation (Variables|Default|GetTarget%20Tile))) (- (.z (Transformation|GetActorLocation (Variables|Default|GetCurrent%20Tile))) _falling)) false false))
        (:Finished
          (Development|PrintString "Game Over"))))))

(event Custom|Drop%20to%20Tile
  (params (Tile%20to%20Drop%20To :type Tile%20Object%20Reference))
  (bind _returnvalue (Transformation|GetActorLocation Tile%20to%20Drop%20To))
  ;[1 1 1] MASTER
  (Variables|Default|SetCurrentZ (.z (Transformation|GetActorLocation self)))
  (bind _playerdropping (Timeline|Timeline_6 PlayFromStart)
    (:Update
      (Transformation|SetActorLocation (Math|Vector|MakeVector (.x _returnvalue) (.y _returnvalue) (+ _playerdropping (Variables|Default|GetCurrentZ))) false false))))

(event Custom|Move%20Right
  (params (Tile%20to%20Move%20to :type Tile%20Object%20Reference))
  (bind _returnvalue (Transformation|GetActorLocation Tile%20to%20Move%20to))
  ;[1 1 1] MASTER
  (Variables|Default|SetCurrentY (.y (Transformation|GetActorLocation self)))
  (bind _movingtoright (Timeline|MoveToRight_TL PlayFromStart)
    (:Update
      (Transformation|SetActorLocation (Math|Vector|MakeVector (.x _returnvalue) (- (Variables|Default|GetCurrentY) _movingtoright) (.z _returnvalue)) false false))))

(event Custom|Move%20Forwards
  (params (Tile%20to%20Move%20to :type Tile%20Object%20Reference))
  (bind _returnvalue (Transformation|GetActorLocation Tile%20to%20Move%20to))
  ;[1 1 1] MASTER
  (Variables|Default|SetCurrentX (.x (Transformation|GetActorLocation self)))
  (bind _movingforward (Timeline|MoveForwards_TL PlayFromStart)
    (:Update
      (Transformation|SetActorLocation (Math|Vector|MakeVector (- (Variables|Default|GetCurrentX) _movingforward) (.y _returnvalue) (.z _returnvalue)) false false))))

(event Custom|SwitchPlayers
  ;[1 1 1] MASTER
  (bind _ascontroller_pawn (Utilities|Casting|CastToControllerPawn (Game|Player|GetPlayerPawn 0)))
  (Variables|Default|SetOrangePlayer (Variables|/Game/Blueprints/ControllerPawn.ControllerPawn_C|GetOrangePawn _ascontroller_pawn))
  (Variables|Default|SetBluePlayer (Variables|/Game/Blueprints/ControllerPawn.ControllerPawn_C|GetBluePawn _ascontroller_pawn))
  (Variables|Default|SetBluePlayerCoords (Transformation|GetActorLocation (Variables|Default|GetBluePlayer)))
  (Variables|Default|SetOrangePlayerCoords (Transformation|GetActorLocation (Variables|Default|GetOrangePlayer)))
  (Variables|Default|SetOrangeCurrentTile (Variables|PlayerPawn_C|GetCurrent%20Tile (Variables|Default|GetOrangePlayer)))
  (Variables|Default|SetBlueCurrentTile (Variables|PlayerPawn_C|GetCurrent%20Tile (Variables|Default|GetBluePlayer)))
  (Transformation|SetActorLocation (Variables|Default|GetOrangePlayer) (Variables|Default|GetBluePlayerCoords) false true)
  (Transformation|SetActorLocation (Variables|Default|GetBluePlayer) (Variables|Default|GetOrangePlayerCoords) false true)
  (Variables|PlayerPawn_C|SetCurrent%20Tile (Variables|Default|GetOrangePlayer) (Variables|Default|GetBlueCurrentTile))
  (Variables|PlayerPawn_C|SetCurrent%20Tile (Variables|Default|GetBluePlayer) (Variables|Default|GetOrangeCurrentTile)))

(event Custom|Move%20Back
  (params (Tile%20to%20Move%20to :type Tile%20Object%20Reference))
  (bind _returnvalue (Transformation|GetActorLocation Tile%20to%20Move%20to))
  ;[1 1 1] MASTER
  (Variables|Default|SetCurrentX (.x (Transformation|GetActorLocation self)))
  (bind _movingbackward (Timeline|MoveBackwards_TL PlayFromStart)
    (:Update
      (Transformation|SetActorLocation (Math|Vector|MakeVector (+ _movingbackward (Variables|Default|GetCurrentX)) (.y _returnvalue) (.z _returnvalue)) false false))))

(fn ConstructionScript
  (Variables|Default|SetcanPlayerMove true))