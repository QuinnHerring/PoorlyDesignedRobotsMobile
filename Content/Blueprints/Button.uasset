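; Floor button that toggles the movement of a linked bridge tile in a puzzle-style level.
; Each trigger overlap runs a FlipFlop that, after a short delay, flips IsPressed and swaps the button's materials between glowing and default.
; It then switches on the tile's DirectionOfMovement, moving the bridge that way when pressed and the opposite way when released by the next overlap.
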(event OnComponentBeginOverlap(Trigger)
  (params (OverlappedComponent :type Primitive%20Component%20Object%20Reference) (OtherActor :type Actor%20Object%20Reference) (OtherComp :type Primitive%20Component%20Object%20Reference) (OtherBodyIndex :type Integer) (bFromSweep :type Boolean) (SweepResult :type Hit%20Result%20Structure%20%28by%20ref%29))
  (bind _affectedbridgetile (Variables|Components|GetAffectedBridgeTile))
  (bind _affectedbridgetile_2 (Variables|Components|GetAffectedBridgeTile))
  (Utilities|FlowControl|FlipFlop
    (:A
      (Utilities|FlowControl|Delay 0.5)
      (Variables|Default|SetisPressed true)
      (Rendering|Material|SetMaterial (Variables|Default|GetButton) 0 "/Game/Textures/EndZones/EndZoneBlueGlow.EndZoneBlueGlow")
      (Rendering|Material|SetMaterial (Variables|Default|GetButton) 2 "/Game/Textures/EndZones/EndZoneBlueGlow.EndZoneBlueGlow")
      (Rendering|Material|SetMaterial (Variables|Default|GetButton) 4 "/Game/Textures/EndZones/EndZoneBlueGlow.EndZoneBlueGlow")
      (switch string (Variables|/Game/Blueprints/Bridge.Bridge_C|GetDirection%20of%20Movement (Variables|Components|GetAffectedBridgeTile))
        (:Up
          (Default|RaiseBridge _affectedbridgetile_2))
        (:Down
          (Default|DropBridge _affectedbridgetile_2))
        (:Forwards
          (Default|MoveBridgeForwards _affectedbridgetile_2))
        (:Back
          (Default|MoveBridgeBackwards _affectedbridgetile_2))
        (:Left
          (Default|MoveBridgeLeft _affectedbridgetile_2))
        (:Right
          (Default|MoveBridgeRight _affectedbridgetile_2))))
    (:B
      (Utilities|FlowControl|Delay 0.5)
      (Variables|Default|SetisPressed false)
      (Rendering|Material|SetMaterial (Variables|Default|GetButton) 0 "/Game/Textures/Top.Top")
      (Rendering|Material|SetMaterial (Variables|Default|GetButton) 2 "/Game/Textures/Side_2.Side_2")
      (Rendering|Material|SetMaterial (Variables|Default|GetButton) 4 "/Game/Textures/Side_1.Side_1")
      (switch string (Variables|/Game/Blueprints/Bridge.Bridge_C|GetDirection%20of%20Movement (Variables|Components|GetAffectedBridgeTile))
        (:Up
          (Default|DropBridge _affectedbridgetile))
        (:Down
          (Default|RaiseBridge _affectedbridgetile))
        (:Forwards
          (Default|MoveBridgeBackwards _affectedbridgetile))
        (:Back
          (Default|MoveBridgeForwards _affectedbridgetile))
        (:Left
          (Default|MoveBridgeRight _affectedbridgetile))
        (:Right
          (Default|MoveBridgeLeft _affectedbridgetile))))))

(fn ConstructionScript
  (|CallParentFunction))