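; Translocator is a button tile that switches players, via the PlayerOnTile reference, when something overlaps its trigger.
; After a short delay, an overlap disables the tile, applies a blue glow to three button material slots and calls SwitchPlayers.
; Ending the overlap re-enables it after the same delay and restores those slots by copying materials from the button's other slots.
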(event OnComponentBeginOverlap(Trigger)
  (params (OverlappedComponent :type Primitive%20Component%20Object%20Reference) (OtherActor :type Actor%20Object%20Reference) (OtherComp :type Primitive%20Component%20Object%20Reference) (OtherBodyIndex :type Integer) (bFromSweep :type Boolean) (SweepResult :type Hit%20Result%20Structure%20%28by%20ref%29))
  (if (not (Variables|Default|GetDisabled))
    (Utilities|FlowControl|Delay 0.49)
    (Variables|Default|SetDisabled true)
    (Rendering|Material|SetMaterial (Variables|Default|GetButton) 4 "/Game/Textures/EndZones/EndZoneBlueGlow.EndZoneBlueGlow")
    (Rendering|Material|SetMaterial (Variables|Default|GetButton) 2 "/Game/Textures/EndZones/EndZoneBlueGlow.EndZoneBlueGlow")
    (Rendering|Material|SetMaterial (Variables|Default|GetButton) 3 "/Game/Textures/EndZones/EndZoneBlueGlow.EndZoneBlueGlow")
    (Default|SwitchPlayers (Variables|Default|GetPlayerOnTile))))

(event OnComponentEndOverlap(Trigger)
  (params (OverlappedComponent :type Primitive%20Component%20Object%20Reference) (OtherActor :type Actor%20Object%20Reference) (OtherComp :type Primitive%20Component%20Object%20Reference) (OtherBodyIndex :type Integer))
  (Utilities|FlowControl|Delay 0.49)
  (Variables|Default|SetDisabled false)
  (Rendering|Material|SetMaterial (Variables|Default|GetButton) 4 (Rendering|Material|GetMaterial (Variables|Default|GetButton) 1))
  (Rendering|Material|SetMaterial (Variables|Default|GetButton) 2 (Rendering|Material|GetMaterial (Variables|Default|GetButton) 6))
  (Rendering|Material|SetMaterial (Variables|Default|GetButton) 3 (Rendering|Material|GetMaterial (Variables|Default|GetButton) 7)))

(fn ConstructionScript
  (|CallParentFunction))