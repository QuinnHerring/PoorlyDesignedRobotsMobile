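; Goal tile for the orange pawn on a tile map, tracking whether that pawn currently stands on it.
; Each Tick it gets the player's ControllerPawn, applies the base orange material to its OrangePawn and compares X and Y positions for exact equality.
; The result switches the tile between glow and base materials and updates the win flags on ControllerPawn and TileMap.
; CanPlayerEnter always allows entry.
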(event EventBeginPlay
  (|CallParentFunction) ; This node is disabled and will not be called.\nDrag off pins to build functionality.
)

(event Collision|EventActorBeginOverlap
  (params (OtherActor :type Actor%20Object%20Reference))
  (|CallParentFunction OtherActor))

(event EventTick
  (params (DeltaSeconds :type Float%20%28single-precision%29))
  (bind _self self)
  (bind _returnvalue (Transformation|GetActorLocation _self))
  (bind (_x _y) (Math|Vector|BreakVector _returnvalue))
  (|CallParentFunction DeltaSeconds)
  (bind _ascontroller_pawn (Utilities|Casting|CastToControllerPawn (Game|Player|GetPlayerPawn 0)))
  (Rendering|Material|SetMaterial (Variables|/Game/Blueprints/PlayerPawn.PlayerPawn_C|GetStaticMesh (Variables|/Game/Blueprints/ControllerPawn.ControllerPawn_C|GetOrangePawn _ascontroller_pawn)) 0 "/Game/Textures/EndZoneBaseOrange.EndZoneBaseOrange")
  (if (and (== _x (.X (Math|Vector|BreakVector (Transformation|GetActorLocation (Variables|/Game/Blueprints/ControllerPawn.ControllerPawn_C|GetOrangePawn _ascontroller_pawn))))) (== _y (.Y (Math|Vector|BreakVector (Transformation|GetActorLocation (Variables|/Game/Blueprints/ControllerPawn.ControllerPawn_C|GetOrangePawn _ascontroller_pawn))))))
    (Rendering|Material|SetMaterial (Variables|Default|GetStaticMesh) 0 "/Game/Textures/EndZoneGlowOrange.EndZoneGlowOrange")
    (Rendering|Material|SetMaterial (Variables|Default|GetStaticMesh) 0 "/Game/Textures/EndZoneGlowOrange.EndZoneGlowOrange")
    (Variables|/Game/Blueprints/ControllerPawn.ControllerPawn_C|SetOrangeNotWon _ascontroller_pawn false)
    (Variables|/Game/Blueprints/TileMap.TileMap_C|SetOrangeWon (Variables|Default|GetTile%20Map self) true)
    (else
      (Rendering|Material|SetMaterial (Variables|Default|GetStaticMesh) 0 "/Game/Textures/EndZoneBaseOrange.EndZoneBaseOrange")
      (Rendering|Material|SetMaterial (Variables|Default|GetStaticMesh) 0 "/Game/Textures/EndZoneBaseOrange.EndZoneBaseOrange")
      (Variables|/Game/Blueprints/ControllerPawn.ControllerPawn_C|SetOrangeNotWon _ascontroller_pawn true)
      (Variables|/Game/Blueprints/TileMap.TileMap_C|SetOrangeWon (Variables|Default|GetTile%20Map self) false))))

(fn ConstructionScript
  (|CallParentFunction))

(fn CanPlayerEnter
  (params (Player%20Pawn :type Player%20Pawn%20Object%20Reference) (From :type Tile%20Object%20Reference))
  (return true))